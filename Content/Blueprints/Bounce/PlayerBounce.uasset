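; Player pawn Blueprint for a physics-driven mesh that bounces off surfaces beneath it and moves on Enhanced Input.
; PlayerMovement pushes the mesh along the control-yaw forward vector, using only the action's X value.
; Tick traces 100 units down and applies an upward velocity-change impulse on every blocking hit.
; Yaw and pitch functions rotate the spring arm and camera but aren't called here; MovePlayer's force logic is disconnected.
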(event Input|EnhancedActionEvents|EnhancedInputActionPlayerMovement
  (params (ActionValue :type Vector%202D%20Structure) (ElapsedSeconds :type Float%20%28double-precision%29) (TriggeredSeconds :type Float%20%28double-precision%29) (InputAction :type Input%20Action%20Object%20Reference :default "/Game/Input/PlayerMovement.PlayerMovement"))
  (Physics|AddForce (Variables|Default|GetStaticMesh) (* (Math|Vector|GetForwardVector (Math|Rotator|MakeRotator 0.0 0.0 (.yaw (Pawn|GetControlRotation :!class /Script/Engine.Pawn)))) (.x ActionValue) (Variables|Default|GetForceStrength)) "None" false))

(event EventBeginPlay
  (Input|AddMappingContext (PlayerController|LocalPlayerSubsystems|GetEnhancedInputLocalPlayerSubsystem (Game|GetPlayerController 0)) "/Game/Input/MyInputMapping.MyInputMapping" 0 "(bIgnoreAllPressedKeysUntilRelease=True,bForceImmediately=False,bNotifyUserSettings=False)"))

(event Collision|EventActorBeginOverlap
  (params (OtherActor :type Actor%20Object%20Reference)))

(event EventTick
  (params (DeltaSeconds :type Float%20%28single-precision%29))
  (bind _staticmesh (Variables|Default|GetStaticMesh))
  (bind _returnvalue (Transformation|GetWorldLocation _staticmesh))
  (bind (_x _y _z) (Math|Vector|BreakVector _returnvalue))
  (bind _outhit (Collision|LineTraceByChannel _returnvalue (Math|Vector|MakeVector _x _y (- _z 1e+02)) "TraceTypeQuery1" false 0 "None"))
  (if true
    (if (.bBlockingHit (Collision|BreakHitResult _outhit))
      (Physics|AddImpulse (Variables|Default|GetStaticMesh) (Math|Vector|MakeVector 0.0 0.0 (Variables|Default|GetBounceStrength)) "None" true))))

(fn ConstructionScript)

(fn MovePlayer
  (params (XOffset :type Float%20%28double-precision%29) (YOffset :type Float%20%28double-precision%29)))

(fn TurnCameraYaw
  (params (AxisValue :type Float%20%28double-precision%29))
  (bind _returnvalue (Utilities|Time|GetWorldDeltaSeconds))
  (bind _cameraturnspeed (Variables|Default|GetCameraTurnSpeed))
  (bind _returnvalue_2 (* AxisValue _cameraturnspeed _returnvalue))
  (Variables|Default|SetCurrentYaw _returnvalue_2)
  (Transformation|AddWorldRotation (Variables|Default|GetSpringArm) (Math|Rotator|MakeRotator 0.0 0.0 _returnvalue_2) false false))

(fn TurnCameraPitch
  (params (AxisValue :type Float%20%28double-precision%29))
  (bind _returnvalue (Utilities|Time|GetWorldDeltaSeconds))
  (bind _cameraturnspeed (Variables|Default|GetCameraTurnSpeed))
  (bind _returnvalue_2 (* AxisValue _cameraturnspeed _returnvalue))
  (Variables|Default|SetCurrentPitch _returnvalue_2)
  (Transformation|AddLocalRotation (Variables|Default|GetCamera) (Math|Rotator|MakeRotator 0.0 _returnvalue_2 0.0) false false))