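; Rings is a collectible ring actor in the Bounce game that counts toward the player's collected total.
; When a PlayerBounce actor overlaps it, PlayerCollide swaps the static mesh material to MI_Cube_03 and increments CollectedRings on player pawn 0.
; An IsRingCollected flag limits the increment to one per ring, while the material is set on every overlap.
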(event EventBeginPlay)

(event Collision|EventActorBeginOverlap
  (params (OtherActor :type Actor%20Object%20Reference))
  (Utilities|Casting|CastToPlayerBounce OtherActor)
  (CallFunction|PlayerCollide))

(event EventTick
  (params (DeltaSeconds :type Float%20%28single-precision%29)))

(fn ConstructionScript)

(fn PlayerCollide
  ;[0.15 0.15 0.15 0.5] Material Change
  (Rendering|Material|SetMaterial (Variables|Default|GetStaticMesh) 0 "/Engine/VREditor/BasicMeshes/MI_Cube_03.MI_Cube_03")
  ;[0.15 0.15 0.15 0.5] Update Collected Rings
  (bind _asplayer_bounce (Utilities|Casting|CastToPlayerBounce (Game|Player|GetPlayerPawn 0)))
  (if (not (Variables|Default|GetIsRingCollected))
    (Variables|/Game/Blueprints/Bounce/PlayerBounce.PlayerBounce_C|SetCollectedRings _asplayer_bounce (+ (Variables|/Game/Blueprints/Bounce/PlayerBounce.PlayerBounce_C|GetCollectedRings _asplayer_bounce) 1))
    (Variables|Default|SetIsRingCollected true)))