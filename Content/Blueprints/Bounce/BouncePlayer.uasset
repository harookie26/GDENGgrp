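; BouncePlayer is a movable actor with a bouncing Sphere component.
; MoveForward and MoveSideward offset the actor along its forward and right vectors by MoveSpeed, without sweep or delta-time scaling.
; Tick calls SmallBounce, which sets the sphere's relative Z from an absolute sine scaled by BounceSpeed and BounceHeight.
; Tick never stores the summed ElapsedTime, and BaseZ, saved at BeginPlay, goes unused.
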(event EventBeginPlay
  (Variables|Default|SetBaseZ (.Z (Math|Vector|BreakVector (Transformation|GetActorLocation)))))

(event EventTick
  (params (DeltaSeconds :type Float%20%28single-precision%29))
  (CallFunction|SmallBounce (+ (Variables|Default|GetElapsedTime) (Utilities|Time|GetWorldDeltaSeconds))))

(fn ConstructionScript)

(fn MoveForward
  (params (Offset :type Float%20%28double-precision%29))
  (Transformation|SetActorLocation (+ (* Offset (Math|Vector|GetForwardVector (Transformation|GetActorRotation)) (Variables|Default|GetMoveSpeed)) (Transformation|GetActorLocation)) false false))

(fn MoveSideward
  (params (Offset :type Float%20%28double-precision%29))
  (Transformation|SetActorLocation (+ (* Offset (Math|Vector|GetRightVector (Transformation|GetActorRotation)) (Variables|Default|GetMoveSpeed)) (Transformation|GetActorLocation)) false false))

(fn SmallBounce
  (params (ElapsedTime :type Float%20%28double-precision%29))
  (bind _sphere (Variables|Default|GetSphere))
  (bind _relativelocation (Variables|/Script/Engine.SceneComponent|GetRelativeLocation _sphere))
  (bind (_x _y) (Math|Vector|BreakVector _relativelocation))
  (Transformation|SetRelativeLocation _sphere (Math|Vector|MakeVector _x _y (* (Math|Float|Absolute(Float) (Math|Trig|Sin(Radians) (* ElapsedTime (Variables|Default|GetBounceSpeed)))) (Variables|Default|GetBounceHeight))) false false))