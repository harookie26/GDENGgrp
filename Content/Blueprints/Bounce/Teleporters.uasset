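; Teleporter actor that moves the PlayerBounce player to its linked PartnerTeleporter on overlap.
; It fires only while the partner is active, then marks itself inactive for TeleporterCooldown, which blocks the partner from sending the player straight back.
; PlayerCollide sets player pawn 0 to the partner's X and Y, keeping the pawn's current Z, without sweeping.
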(event EventBeginPlay)

(event Collision|EventActorBeginOverlap
  (params (OtherActor :type Actor%20Object%20Reference))
  (Utilities|Casting|CastToPlayerBounce OtherActor)
  (if (Variables|Teleporters_C|GetIsActive (Variables|Default|GetPartnerTeleporter))
    (Variables|Default|SetIsActive false)
    (CallFunction|PlayerCollide)
    (Utilities|FlowControl|Delay (Variables|Default|GetTeleporterCooldown))
    (Variables|Default|SetIsActive true)))

(fn ConstructionScript)

(fn PlayerCollide
  (bind _returnvalue (Game|Player|GetPlayerPawn 0))
  (bind _partnerteleporter (Variables|Default|GetPartnerTeleporter))
  (bind _returnvalue_2 (Transformation|GetActorLocation _partnerteleporter))
  (bind (_x _y) (Math|Vector|BreakVector _returnvalue_2))
  (Transformation|SetActorRelativeLocation _returnvalue (Math|Vector|MakeVector _x _y (.Z (Math|Vector|BreakVector (Transformation|GetActorLocation _returnvalue))))))